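; Camera origin actor that places the player's camera pawn at an angle and distance from itself, looking back at the origin.
; The construction script finds or spawns the BP_CameraPawn and moves it to the computed transform, so placement updates in the editor.
; On BeginPlay it spawns the pawn if none is cached, has player controller 0 possess it, and attaches it to the origin.
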(event EventBeginPlay
  ;[0.15 0.15 0.15 0.5] If the camera origin has the camera pawn cached, set it as the main player
  (Variables|Internal|GetCameraPawn
    (:then
      _)
    (:else
      (bind _returnvalue (Game|SpawnActorfromClass "/Game/MonumentValley/Blueprints/Pawn/BP_CameraPawn.BP_CameraPawn_C" (CallFunction|GetCameraTransform) "Undefined" "MultiplyWithRoot" 0 0))
      (Variables|Internal|SetCameraPawn _returnvalue)))
  (Pawn|Possess (Game|GetPlayerController 0) (Variables|Internal|GetCameraPawn))
  (Transformation|AttachActorToActor (Variables|Internal|GetCameraPawn) self "None" "KeepWorld" "KeepWorld" "KeepWorld" true))

(fn ConstructionScript
  ;[0.15 0.15 0.15 0.5] Updates the camera location on construct
  (Config|UpdateCameraLocation))

(fn GetCameraTransform
  (bind _returnvalue (Transformation|GetActorForwardVector))
  (bind _returnvalue_2 (Transformation|GetActorLocation))
  (bind _distancefromorigin (Variables|Config|GetDistanceFromOrigin))
  (bind _cameraangle (Variables|Config|GetCameraAngle))
  (bind _returnvalue_3 (Math|Vector|RotateVector _returnvalue _cameraangle))
  (bind _returnvalue_4 (* _returnvalue_3 _distancefromorigin))
  (bind _returnvalue_5 (+ _returnvalue_2 _returnvalue_4))
  ;[0.15 0.15 0.15 0.5] Gets the required transform of the player's camera
  (return (Math|Transform|MakeTransform _returnvalue_5 (Math|Rotator|FindLookatRotation _returnvalue_5 (Transformation|GetActorLocation)))))

(fn UpdateCameraLocation
  (bind _returnvalue (CallFunction|GetCameraTransform))
  ;[0.15 0.15 0.15 0.5] Checks if the CameraPawn exists, relocates and caches it. If not, spawns it in and caches the newly spawned actor
  (bind _returnvalue_2 (Actor|GetActorOfClass "/Game/MonumentValley/Blueprints/Pawn/BP_CameraPawn.BP_CameraPawn_C"))
  (Utilities|IsValid _returnvalue_2
    (:Is%20Valid
      (bind _output_get (Variables|Internal|SetCameraPawn _returnvalue_2))
      (Transformation|SetActorTransform _output_get _returnvalue))
    (:Is%20Not%20Valid
      (bind _returnvalue_3 (Game|SpawnActorfromClass "/Game/MonumentValley/Blueprints/Pawn/BP_CameraPawn.BP_CameraPawn_C" _returnvalue "Undefined" "MultiplyWithRoot" 0 0))
      (Variables|Internal|SetCameraPawn _returnvalue_3))))