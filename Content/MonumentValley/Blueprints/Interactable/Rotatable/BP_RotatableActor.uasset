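; Touch-rotatable puzzle actor that the player drags around one chosen axis, changing which grid tiles connect in a Monument Valley-style level.
; Drags project the touch onto a plane normal to that axis and apply the signed angle delta as local rotation.
; On release, it locks interaction while a timeline eases it to the nearest snap multiple.
; Tile links reset on touch, then update from the snapped rotation state once snapping finishes.
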(event Custom|UpdateTileLinks
  (params (NewState :type E_RotatableActorStates%20Enum :default "NewEnumerator0"))
  ;[0.15 0.15 0.15 0.5] Dynamically updates the TravelableTiles array of the point depending on the new location state of the actor
  (bind (_keypin _valuepin) (Utilities|Map|ForEachLoop(Map) (Variables|Config|GetTileLinkMap))
    (:then
      (for _array_element (.links _valuepin)
        (Default|ToggleContains (.gridpoint _array_element) (Utilities|Enum|Equal(Enum) _keypin NewState) (.linkto _array_element))
        (Default|ToggleContains (.linkto _array_element) (Utilities|Enum|Equal(Enum) _keypin NewState) (.gridpoint _array_element))
        (Default|DebugAllConnections (.gridpoint _array_element))))))

(event EventInteractableTouchReleased
  (bind _snapanglemultiple (Variables|Config|GetSnapAngleMultiple))
  (bind _rotationaxis (Variables|Config|GetRotationAxis))
  (bind _returnvalue (Getters|GetAxisValue _rotationaxis))
  (bind _returnvalue_2 (/ _returnvalue _snapanglemultiple))
  (bind _returnvalue_3 (Math|Float|Round _returnvalue_2))
  ;[0.15 0.15 0.15 0.5] Snaps the actor's rotation to the closest angle specified by the SnapAngleMultiple variable
  (CallFunction|InteractableLockInteraction self true)
  (Variables|Snapping|SetRotationStateAfterSnapping (.Value (Utilities|Map|Find (Variables|Snapping|GetRotationStateMap) _returnvalue_3)))
  (Variables|Snapping|SetSnapAngle (* (Variables|Config|GetSnapAngleMultiple) _returnvalue_3))
  (bind _angleprogression (Timeline|Timeline PlayFromStart)
    (:Update
      ;;[0 0 0 0.5] Rotates the released actor towards the nearest 90 degree angle
      (Variables|Snapping|SetRotationSnapDeltaTime (+ (Variables|Snapping|GetRotationSnapDeltaTime) _angleprogression))
      (RotationSetting|SetAxisValue (Variables|Config|GetRotationAxis) (Math|Interpolation|FInterpTo (Getters|GetAxisValue (Variables|Config|GetRotationAxis)) (Variables|Snapping|GetSnapAngle) (Variables|Snapping|GetRotationSnapDeltaTime) 1.0)))
    (:Finished
      ;;[0 0 0 0.5] Enables the interaction, resets the deltaTime and updates the tile path links
      (CallFunction|InteractableLockInteraction self false)
      (Variables|Snapping|SetRotationSnapDeltaTime 0.0)
      (CallFunction|UpdateTileLinks (Variables|Snapping|GetRotationStateAfterSnapping)))))

(event EventInteractableTouchOngoing
  (params (RawInputPos :type Vector%202D%20Structure))
  (bind _returnvalue (Math|GetTouchAngle RawInputPos))
  ;[0.15 0.15 0.15 0.5] Updates the rotation of the actor
  (RotationSetting|AddAngletoAxis (Variables|Config|GetRotationAxis) (- _returnvalue (Variables|Internal|GetCurrentAngle)))
  (Variables|Internal|SetCurrentAngle _returnvalue))

(fn ConstructionScript)

(fn GetDirectionTowardsCamera
  ;[0.15 0.15 0.15 0.5] Gets the normalized direction from the actor to the camera
  (return (Math|Vector|GetUnitDirection(Vector) (Transformation|GetActorLocation) (Camera|GetCameraLocation (Game|GetPlayerCameraManager 0)))))

(fn GetAxisValue
  (params (Axis :type E_RotationAxis%20Enum :default "NewEnumerator0"))
  (bind _returnvalue (Getters|GetRelativeRotation))
  ;[0.15 0.15 0.15 0.5] Gets the rotation value of the given axis
  (return (Utilities|Select :Index Axis :NewEnumerator0 0.0 :NewEnumerator1 (.roll _returnvalue) :NewEnumerator2 (.pitch _returnvalue) :NewEnumerator3 (.yaw _returnvalue))))

(fn GetTouchAngle
  (params (ScreenPosition :type Vector%202D%20Structure%20%28by%20ref%29))
  (bind _returnvalue (Transformation|GetActorLocation))
  (bind _returnvalue_2 (Game|GetPlayerController 0))
  (bind _returnvalue_3 (Transformation|GetActorLocation))
  (bind _rotationaxis (Variables|Config|GetRotationAxis))
  (bind _rotationaxis_2 (Variables|Config|GetRotationAxis))
  (bind _returnvalue_4 (Getters|GetAxisNormal _rotationaxis_2))
  (bind _returnvalue_5 (Getters|GetAxisNormal _rotationaxis))
  (bind _intersection (CallFunction|ScreentoWorldIntersectPoint _returnvalue_2 ScreenPosition 5e+04 _returnvalue_3 _returnvalue_4))
  (bind _returnvalue_6 (Math|Rotator|MakeRotfromX _returnvalue_5))
  (bind _returnvalue_7 (Math|Vector|GetRightVector _returnvalue_6))
  (bind _returnvalue_8 (Math|Vector|GetUnitDirection(Vector) _returnvalue _intersection))
  (bind _returnvalue_9 (Math|Vector|DotProduct _returnvalue_7 _returnvalue_8))
  (bind _returnvalue_10 (Class|KismetMathLibrary|DegAcos _returnvalue_9))
  ;[0.15 0.15 0.15 0.5] Gets the angle of the touch position projected on a plane projected from the actor's origin facing the camera
  (return (Math|Float|SelectFloat _returnvalue_10 (* _returnvalue_10 -1.0) (< (Math|Vector|DotProduct (Math|Vector|GetUpVector _returnvalue_6) _returnvalue_8) 0.0))))

(fn AddAngletoAxis
  (params (Axis :type E_RotationAxis%20Enum :default "NewEnumerator0") (Angle :type Float%20%28double-precision%29))
  ;[0.15 0.15 0.15 0.5] Adds the given angle to the given axis's value
  (switch Utilities|FlowControl|Switch|SwitchonE_RotationAxis Axis
    (:NewEnumerator0
      _)
    (:NewEnumerator1
      (Transformation|AddActorLocalRotation (Math|Rotator|MakeRotator Angle 0.0 0.0) false false))
    (:NewEnumerator2
      (Transformation|AddActorLocalRotation (Math|Rotator|MakeRotator 0.0 Angle 0.0) false false))
    (:NewEnumerator3
      (Transformation|AddActorLocalRotation (Math|Rotator|MakeRotator 0.0 0.0 (* Angle -1.0)) false false)))
  (return))

(fn SetAxisValue
  (params (Axis :type E_RotationAxis%20Enum :default "NewEnumerator0") (Angle :type Float%20%28double-precision%29))
  (bind _returnvalue (Getters|GetRelativeRotation))
  (bind _returnvalue_2 (Getters|GetRelativeRotation))
  (bind _returnvalue_3 (Getters|GetRelativeRotation))
  ;[0.15 0.15 0.15 0.5] Sets the rotational angle on the given axis
  (Transformation|SetActorRelativeRotation (Utilities|Select :Index Axis :NewEnumerator0 "0, 0, 0" :NewEnumerator1 (Math|Rotator|MakeRotator Angle (.pitch _returnvalue_2) (.yaw _returnvalue_2)) :NewEnumerator2 (Math|Rotator|MakeRotator (.roll _returnvalue_3) Angle (.yaw _returnvalue_3)) :NewEnumerator3 (Math|Rotator|MakeRotator (.roll _returnvalue) (.pitch _returnvalue) Angle)))
  (return))

(fn GetAxisNormal
  (params (Axis :type E_RotationAxis%20Enum :default "NewEnumerator0"))
  ;[0.15 0.15 0.15 0.5] Gets the actor normal depending on the given axis
  (return (Utilities|Select :Index Axis :NewEnumerator0 "0, 0, 0" :NewEnumerator1 (Transformation|GetActorForwardVector) :NewEnumerator2 (Transformation|GetActorRightVector) :NewEnumerator3 (Transformation|GetActorUpVector))))

(fn GetRelativeRotation
  ;[0.15 0.15 0.15 0.5] Gets the actor's relative rotation
  (return (.rotation (Transformation|GetRelativeTransform (Variables|Default|GetDefaultSceneRoot)))))

(fn InteractableonTouched
  (params (ImpactPoint :type Vector :default "0, 0, 0") (RawInputPos :type Vector%202D%20Structure))
  ;[0.15 0.15 0.15 0.5] Returns that it is a valid interactable and saves the starting angle between the base and
  (if (CallFunction|IsInteractionLocked)
    (return false)
    (else
      (Variables|Internal|SetCurrentAngle (Math|GetTouchAngle RawInputPos))
      (CallFunction|UpdateTileLinks "NewEnumerator0")
      (return true))))