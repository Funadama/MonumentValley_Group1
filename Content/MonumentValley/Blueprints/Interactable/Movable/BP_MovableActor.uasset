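; Draggable puzzle piece that slides along one chosen axis and updates walkable tile links to match its position.
; A handle spawned at BeginPlay becomes its parent and anchor for relative movement.
; Touch input is intersected with an axis-based plane, rotated to stabilize the delta, and clamped to a step range.
; Touching requests link removal; releasing animates a snap to the nearest step, then updates that step's TileLinkMap connections.
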(event Custom|UpdateTilePath
  (params (NewValue :type Integer))
  ;[0.15 0.15 0.15 0.5] Update Tile Links
  ;;[0 0 0] Disconect all nodes that where connected
  (for _array_element (.links (.Value (Utilities|Map|Find (Variables|Config|GetTileLinkMap) (Variables|Default|GetNew%20Value))))
    (Default|ToggleContains (.gridpoint _array_element) false 0 (.linkto _array_element))
    (Default|ToggleContains (.linkto _array_element) false 0 (.gridpoint _array_element)))
  ;;[0 0 0] Connect the nodes on the new value
  (for _array_element_2 (.links (.Value (Utilities|Map|Find (Variables|Config|GetTileLinkMap) NewValue)))
    (Default|ToggleContains (.gridpoint _array_element_2) true 0 (.linkto _array_element_2))
    (Default|ToggleContains (.linkto _array_element_2) true 0 (.gridpoint _array_element_2)))
  (Variables|Default|SetNew%20Value NewValue)
  (CallFunction|DebugAllConnections))

(event EventInteractableTouchOngoing
  (params (RawInputPos :type Vector%202D%20Structure))
  ;[0.15 0.15 0.15 0.5] Updates the actor's location based on the movement of the input and starting location
  (bind _output_get (Variables|Internal|SetCurrentMoveValue (Getters|GetNewLocationValue (- (CallFunction|ScreentoWorldIntersectPoint (Game|GetPlayerController 0) RawInputPos 5e+04 (Transformation|GetActorLocation (Variables|Internal|GetHandle)) (Getters|GetRelativeAxisNormal (Variables|Config|GetMoveAxis))) (Variables|Internal|GetInputOrigin)) (Variables|Config|GetMoveAxis))))
  (Location|SetValueonAxis _output_get (Variables|Config|GetMoveAxis)))

(event EventInteractableTouchReleased
  ;[0.15 0.15 0.15 0.5] When released, snap the movement value to the closest increment of the StepSize
  (Variables|Conditions|SetIsActive false)
  (Variables|Snapping|SetSnapLocation (* (Math|Float|Round (/ (Variables|Internal|GetCurrentMoveValue) (Variables|Config|GetMoveStepSize))) (Variables|Config|GetMoveStepSize)))
  (bind _moveprogression (Timeline|Timeline PlayFromStart)
    (:Update
      (Location|SetValueonAxis (+ (* _moveprogression (- (Variables|Snapping|GetSnapLocation) (Variables|Internal|GetCurrentMoveValue))) (Variables|Internal|GetCurrentMoveValue)) (Variables|Config|GetMoveAxis)))
    (:Finished
      ;;[0 0 0 0.5] Reactivate the actor and set new current location
      (Variables|Conditions|SetIsActive true)
      (bind _output_get (Variables|Internal|SetCurrentMoveValue (Variables|Snapping|GetSnapLocation)))
      (CallFunction|UpdateTilePath (Math|Float|Round (/ _output_get (Variables|Config|GetMoveStepSize)))))))

(event EventBeginPlay
  (bind _returnvalue (Actor|GetAttachParentActor))
  (bind _returnvalue_2 (Transformation|GetActorTransform))
  ;[0.15 0.15 0.15 0.5] Spawns in a handle to be used as an anchor to move along it's axes
  (bind _returnvalue_3 (Game|SpawnActorfromClass "/Game/MonumentValley/Blueprints/Interactable/Handle/BP_InteractableHandle.BP_InteractableHandle_C" (Math|Transform|MakeTransform (.location _returnvalue_2) (.rotation _returnvalue_2) "1.000000,1.000000,1.000000") "Undefined" "MultiplyWithRoot" 0 0))
  (bind _output_get (Variables|Internal|SetHandle _returnvalue_3))
  (Utilities|IsValid _returnvalue
    (:Is%20Valid
      (Transformation|AttachActorToActor _output_get _returnvalue "None" "KeepWorld" "KeepWorld" "KeepWorld" true))
    (:Is%20Not%20Valid
      _))
  (Transformation|AttachActorToActor (Variables|Internal|GetHandle) "None" "KeepWorld" "KeepWorld" "KeepWorld" true))

(fn ConstructionScript)

(fn GetNewLocationValue
  (params (InputDelta :type Vector) (Axis :type E_MovementAxis%20Enum :default "NewEnumerator0"))
  (bind _movestepsize (Variables|Config|GetMoveStepSize))
  (bind _steprange (Variables|Config|GetStepRange))
  (bind _l_xaxis (LocalVariables|GetL_XAxis))
  (bind _l_yaxis (LocalVariables|GetL_YAxis))
  (bind _moveaxis (Variables|Config|GetMoveAxis))
  (bind _moveaxis_2 (Variables|Config|GetMoveAxis))
  (bind _returnvalue (Getters|GetRelativeAxisNormal _moveaxis_2))
  (bind _returnvalue_2 (Utilities|Select :Index _moveaxis :NewEnumerator0 "0, 0, 0" :NewEnumerator1 _l_yaxis :NewEnumerator2 _l_xaxis :NewEnumerator3 _l_xaxis))
  (bind _rotatedvector (CallFunction|RotateVectortoNormal _returnvalue _returnvalue_2 InputDelta))
  (bind (_x _y _z) (Math|Vector|BreakVector _rotatedvector))
  (bind _returnvalue_3 (Utilities|Select :Index Axis :NewEnumerator0 0.0 :NewEnumerator1 _x :NewEnumerator2 _y :NewEnumerator3 _z))
  ;[0.15 0.15 0.15 0.5] Gets the input value used for the axis
  (return (Math|Float|Clamp(Float) (+ (select (and (Utilities|Operators|EqualEqual (Math|Vector|NegateVector _returnvalue) _returnvalue_2 0.001) (Utilities|Enum|Equal(Enum) (Variables|Config|GetMoveAxis) "NewEnumerator3")) (* _returnvalue_3 -1.0) _returnvalue_3) (Variables|Internal|GetInputStartMoveValue)) (* (* (.stepcountback _steprange) _movestepsize) -1.0) (* (.stepcountforward _steprange) _movestepsize))))

(fn GetRelativeAxisNormal
  (params (Axis :type E_MovementAxis%20Enum :default "NewEnumerator0"))
  (bind _returnvalue (Transformation|GetActorRightVector))
  ;[0.15 0.15 0.15 0.5] Gets the normal on a specific axis
  (return (Utilities|Select :Index Axis :NewEnumerator0 "0, 0, 0" :NewEnumerator1 _returnvalue :NewEnumerator2 (Transformation|GetActorForwardVector) :NewEnumerator3 _returnvalue)))

(fn SetValueonAxis
  (params (NewValue :type Float%20%28double-precision%29) (Axis :type E_MovementAxis%20Enum :default "NewEnumerator0"))
  ;[0.15 0.15 0.15 0.5] Sets the relative location on the given axis
  (Transformation|SetActorRelativeLocation (* (Utilities|Select :Index Axis :NewEnumerator0 "0, 0, 0" :NewEnumerator1 "1.000000,0.000000,0.000000" :NewEnumerator2 "0.000000,1.000000,0.000000" :NewEnumerator3 "0.000000,0.000000,1.000000") NewValue))
  (return))

(fn InteractableonTouched
  (params (ImpactPoint :type Vector :default "0, 0, 0") (RawInputPos :type Vector%202D%20Structure))
  ;[0.15 0.15 0.15 0.5] Checks if the actor is active. If true, caches the input origin and the current move value as the starting value
  (if (Variables|Conditions|GetIsActive)
    ;;[0 0 0 0.5] Calls OnLocationChanged with an invalid index to remove any connection during interaction
    (CallFunction|UpdateTilePath (+ (.stepcountforward (Variables|Config|GetStepRange)) 1))
    (Variables|Internal|SetInputOrigin (CallFunction|ScreentoWorldIntersectPoint (Game|GetPlayerController 0) RawInputPos 5e+04 (Transformation|GetActorLocation (Variables|Internal|GetHandle)) (Getters|GetRelativeAxisNormal (Variables|Config|GetMoveAxis))))
    (Variables|Internal|SetInputStartMoveValue (Variables|Internal|GetCurrentMoveValue))
    (return true)
    (else
      (return false))))