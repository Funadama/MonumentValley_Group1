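; BP_InteractableActor appears to be a base actor for touch-interactable objects in the Monument Valley game, with support for locking interaction.
; When ShouldDisableOnPlayerStep is set, lock events add or remove the calling actor in LockSet.
; IsInteractionLocked reports true while any actor remains in the set, so several lockers can overlap safely.
; The default touch handler does nothing and returns false.
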(event EventBeginPlay)

(event EventInteractableLockInteraction
  (params (LockingActor :type Actor%20Object%20Reference%20%28by%20ref%29) (isLocking :type Boolean))
  (bind _lockset (Variables|Locking|GetLockSet))
  ;[0.15 0.15 0.15 0.5] Adds/Removes actors from the lock set
  (if (Variables|Locking|GetShouldDisableOnPlayerStep)
    (if isLocking
      (Utilities|Set|Add _lockset LockingActor)
      (else
        (Utilities|Set|Remove _lockset LockingActor)))))

(fn ConstructionScript)

(fn IsInteractionLocked
  ;[0.15 0.15 0.15 0.5] Returns true if the lock set contains at least one element
  (return (Utilities|Set|IsNotEmpty (Variables|Locking|GetLockSet))))

(fn InteractableonTouched
  (params (ImpactPoint :type Vector :default "0, 0, 0") (RawInputPos :type Vector%202D%20Structure))
  (return false))