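; Draggable Monument Valley actor that slides along one axis within a clamped range as the player touches and drags it.
; Touch input is deprojected onto a camera-facing plane, and its delta is flattened onto an axis-specific plane for stable movement, then offset from the drag's starting value.
; On release, a timeline eases it to the nearest snap increment while input is disabled, then broadcasts the snapped step index.
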(event EventInteractableTouchOngoing
  (params (RawInputPos :type Vector%202D%20Structure))
  ;[0.15 0.15 0.15 0.5] Updates the actor's location based on the movement of the input and starting location
  (bind _positiononactorplane (Getters|ProjectInputonPlane RawInputPos))
  (bind _newvalue (Getters|GetNewLocationValue (- _positiononactorplane (Variables|Internal|GetInputOrigin)) (Variables|Config|GetMoveAxis)))
  (bind _output_get (Variables|Internal|SetCurrentMoveValue _newvalue))
  (Location|SetValueonAxis _output_get (Variables|Config|GetMoveAxis)))

(event EventInteractableTouchReleased
  ;[0.15 0.15 0.15 0.5] When released, snap the movement value to the closest increment of the MoveSnapMultiple variable
  (Variables|Conditions|SetIsActive false)
  (Variables|Snapping|SetSnapLocation (* (Math|Float|Round (/ (Variables|Internal|GetCurrentMoveValue) (Variables|Config|GetMoveSnapMultiple))) (Variables|Config|GetMoveSnapMultiple)))
  (bind _moveprogression (Timeline|Timeline PlayFromStart)
    (:Update
      (Location|SetValueonAxis (+ (* _moveprogression (- (Variables|Snapping|GetSnapLocation) (Variables|Internal|GetCurrentMoveValue))) (Variables|Internal|GetCurrentMoveValue)) (Variables|Config|GetMoveAxis)))
    (:Finished
      ;;[0 0 0 0.5] Reactivate the actor and set new current location
      (Variables|Conditions|SetIsActive true)
      (bind _output_get (Variables|Internal|SetCurrentMoveValue (Variables|Snapping|GetSnapLocation)))
      (Default|CallOnLocationChanged (Math|Float|Round (/ _output_get (Variables|Config|GetMoveSnapMultiple)))))))

(event EventBeginPlay
  ;[0.15 0.15 0.15 0.5] Caches the origin location of the actor
  (Variables|Internal|SetOriginLocation (Transformation|GetActorLocation)))

(fn ConstructionScript)

(fn GetDirectionTowardsCamera
  ;[0.15 0.15 0.15 0.5] Gets the normalized direction from the actor to the camera
  (return (Math|Vector|GetUnitDirection(Vector) (Variables|Internal|GetOriginLocation) (Camera|GetCameraLocation (Game|GetPlayerCameraManager 0)))))

(fn GetAxisValue
  (params (Axis :type E_MovementAxis%20Enum :default "NewEnumerator0"))
  (bind _returnvalue (Transformation|GetActorLocation))
  ;[0.15 0.15 0.15 0.5] Gets the location value of the given axis
  (return (Utilities|Select :Index Axis :NewEnumerator0 0.0 :NewEnumerator1 (.x _returnvalue) :NewEnumerator2 (.y _returnvalue) :NewEnumerator3 (.z _returnvalue))))

(fn GetNewLocationValue
  (params (InputDelta :type Vector) (Axis :type E_MovementAxis%20Enum :default "NewEnumerator0"))
  (bind _moverange (Variables|Config|GetMoveRange))
  (bind _l_xaxis (LocalVariables|GetL_XAxis))
  (bind _l_yaxis (LocalVariables|GetL_YAxis))
  (bind _returnvalue (Utilities|Select :Index Axis :NewEnumerator0 "0, 0, 0" :NewEnumerator1 _l_yaxis :NewEnumerator2 _l_xaxis :NewEnumerator3 _l_yaxis))
  (bind _returnvalue_2 (Math|Vector|ProjectVectorontoPlane InputDelta _returnvalue))
  ;[0.15 0.15 0.15 0.5] Gets the input value used for the axis
  ;;[0 0 0 0.5] Adjusts the new position value depending on the starting value
  (return (Math|Float|Clamp(Float) (+ (* (Utilities|Select :Index Axis :NewEnumerator0 0.0 :NewEnumerator1 (.x _returnvalue_2) :NewEnumerator2 (.y _returnvalue_2) :NewEnumerator3 (.z _returnvalue_2)) (Variables|Config|GetDragSpeedMultiplier)) (Variables|Internal|GetInputStartMoveValue)) (.min _moverange) (.max _moverange))))

(fn ProjectInputonPlane
  (params (ScreenPosition :type Vector%202D%20Structure%20%28by%20ref%29))
  ;[0.15 0.15 0.15 0.5] Gets the position of the input where it intersects with the plane towards the camera
  (return (Class|KismetMathLibrary|ProjectPointontoPlane (.WorldPosition (Class|GameplayStatics|DeprojectScreentoWorld (Game|GetPlayerController 0) ScreenPosition)) (Variables|Internal|GetInputOrigin) (Getters|GetDirectionTowardsCamera))))

(fn SetValueonAxis
  (params (NewValue :type Float%20%28double-precision%29) (Axis :type E_MovementAxis%20Enum :default "NewEnumerator0"))
  (bind _returnvalue (Transformation|GetActorLocation))
  (bind _returnvalue_2 (Transformation|GetActorLocation))
  (bind _returnvalue_3 (Transformation|GetActorLocation))
  ;[0.15 0.15 0.15 0.5] Sets the location on the given axis to the given value
  (Transformation|SetActorLocation (Utilities|Select :Index Axis :NewEnumerator0 "0, 0, 0" :NewEnumerator1 (Math|Vector|MakeVector (+ (.x (Variables|Internal|GetOriginLocation)) NewValue) (.y _returnvalue_2) (.z _returnvalue_2)) :NewEnumerator2 (Math|Vector|MakeVector (.x _returnvalue_3) (+ NewValue (.y (Variables|Internal|GetOriginLocation))) (.z _returnvalue_3)) :NewEnumerator3 (Math|Vector|MakeVector (.x _returnvalue) (.y _returnvalue) (+ NewValue (.z (Variables|Internal|GetOriginLocation))))) false false)
  (return))

(fn InteractableonTouched
  (params (ImpactPoint :type Vector :default "0, 0, 0") (RawInputPos :type Vector%202D%20Structure))
  ;[0.15 0.15 0.15 0.5] Checks if the actor is active. If true, caches the input origin and the current move value as the starting value
  (if (Variables|Conditions|GetIsActive)
    (bind _positiononactorplane (Getters|ProjectInputonPlane RawInputPos))
    (Variables|Internal|SetInputOrigin _positiononactorplane)
    (Variables|Internal|SetInputStartMoveValue (Variables|Internal|GetCurrentMoveValue))
    (return true)
    (else
      (return false))))