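; BP_CameraPawn is the player pawn that turns touch or mouse input into interactions with world actors.
; It adds the mobile Enhanced Input mapping and resolves screen position, substituting the cursor position when mouse input is detected.
; On press, a visibility trace from that position messages the hit actor, caching it if it responds.
; The cached actor receives ongoing and release messages, then is cleared when input completes or cancels.
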(event Custom|TouchCompleted
  ;[0.15 0.15 0.15 0.5] Calls Interactable_Touch_Released on the selected actor and clears the reference
  (bind _currentselectedactor (Variables|Default|GetCurrentSelectedActor)
    (:then
      (Class|BPIInteractable|InteractableTouchReleased(Message) _currentselectedactor)
      (Variables|Default|SetCurrentSelectedActor 0))
    (:else)))

(event Custom|TriggeredTouch
  (params (RawInputPos :type Vector%202D%20Structure))
  (bind (_x _y) (Math|Vector2D|BreakVector2D RawInputPos))
  (bind _returnvalue (Game|GetPlayerController 0))
  (bind (_worldlocation _worlddirection) (Class|PlayerController|DeprojectScreenPositiontoWorld _returnvalue _x _y))
  (bind (_start _end) (Utilities|GetDirectionalLine _worldlocation _worlddirection 5e+03))
  ;[0.15 0.15 0.15 0.5] On starting a touch input, check if the player has touched on any interactable actor with a raycast. If true, cache a reference to the actor
  (bind (_outhit _returnvalue_2) (Collision|LineTraceByChannel _start _end "TraceTypeQuery1" false 0 "None" true "(R=0.135355,G=0.141628,B=1.000000,A=1.000000)" "(R=0.000000,G=1.000000,B=0.000000,A=1.000000)" 1.0))
  (if _returnvalue_2
    (bind _isvalid (Class|BPIInteractable|InteractableonTouched(Message) (.HitActor (Collision|BreakHitResult _outhit)) (.ImpactPoint (Collision|BreakHitResult _outhit)) RawInputPos))
    (if _isvalid
      (Variables|Default|SetCurrentSelectedActor (.HitActor (Collision|BreakHitResult _outhit))))))

(event Custom|TouchOngoing
  (params (RawInputPos :type Vector%202D%20Structure))
  ;[0.15 0.15 0.15 0.5] Calls Interactable_Touch_Ongoing on the selected actor if it is valid
  (bind _currentselectedactor (Variables|Default|GetCurrentSelectedActor)
    (:then
      (Class|BPIInteractable|InteractableTouchOngoing(Message) _currentselectedactor RawInputPos))
    (:else)))

(event Input|EnhancedActionEvents|EnhancedInputActionIA_Touch_Down
  (params (ActionValue :type Vector :default "0, 0, 0") (ElapsedSeconds :type Float%20%28double-precision%29) (TriggeredSeconds :type Float%20%28double-precision%29) (InputAction :type Input%20Action%20Object%20Reference :default "/Game/MonumentValley/Input/Actions/IA_Touch_Down.IA_Touch_Down"))
  (bind _returnvalue (CallFunction|GetInputPosition ActionValue))
  ;[0.15 0.15 0.15 0.5] Handles touch input
  (:Started
    (CallFunction|TriggeredTouch _returnvalue))
  (:Ongoing
    (CallFunction|TouchOngoing _returnvalue))
  (:Canceled
    (CallFunction|TouchCompleted :!label _label) ; Canceled: Mobile Input\nCompleted: Mouse Input
  )
  (:Completed
    (goto _label)))

(event EventBeginPlay
  (bind _returnvalue (Game|GetPlayerController 0))
  ;[0.15 0.15 0.15 0.5] Adds the touch controls mapping to the player
  (Variables|/Script/Engine.PlayerController|SetbShowMouseCursor _returnvalue true)
  (Input|AddMappingContext (PlayerController|LocalPlayerSubsystems|GetEnhancedInputLocalPlayerSubsystem _returnvalue) "/Game/MonumentValley/Input/IMC_MobileInput.IMC_MobileInput" 1 "(bIgnoreAllPressedKeysUntilRelease=True,bForceImmediately=False,bNotifyUserSettings=False)"))

(fn ConstructionScript)

(fn GetInputPosition
  (params (InputPin :type Vector))
  (bind _returnvalue (Game|GetPlayerController 0))
  (bind (_locationx _locationy) (Game|Player|GetMousePosition _returnvalue))
  ;[0.15 0.15 0.15 0.5] Gets the mouse position when mouse input is detected, otherwise return the given input
  (return (Math|Conversions|ToVector2D(Vector) (Math|Vector|SelectVector InputPin (Math|Vector|MakeVector _locationx _locationy 0.0) (Utilities|Operators|NotEqual(!=) InputPin "1.000000,0.000000,0.000000" 0.001)))))