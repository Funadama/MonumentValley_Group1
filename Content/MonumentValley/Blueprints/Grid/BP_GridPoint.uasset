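; BP_GridPoint is a grid node that stores the other points that can be travelled to from it.
; Its construction script redraws every point's links outside distribution builds, with white lines for two-way links and yellow arrows for one-way.
; A map of already processed points prevents drawing two-way links twice.
; ToggleContains adds or removes a link on behalf of a utility Blueprint, which cannot edit the array itself.
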(fn ConstructionScript
  (TravelPoints|DebugAllConnections))

(fn DebugAllConnections
  ;[0.15 0.15 0.15 0.5] Clear Debug data
  (if (not (Class|KismetSystemLibrary|IsPackagedforDistribution))
    (Rendering|Debug|FlushPersistentDebugLines)
    (Utilities|Map|Clear (LocalVariables|GetL_DebuggedPoints))
    ;[0.15 0.15 0.15 0.5] Debugs all the TravelPoint connections, checking whether they have already been debugged from one to another. If the connection is bidirectional, it’s shown in a different color.
    ; Uses a Map<Array> that holds what lines have been debugged
    (bind _outactors (Actor|GetAllActorsOfClass "BP_GridPoint_C"))
    (for _array_element _outactors
      (Utilities|Array|Clear (LocalVariables|GetL_GridArray))
      (for _array_element_2 (TravelPoints|GetTravelablePoints _array_element)
        (Utilities|IsValid _array_element_2
          (:Is%20Valid
            (Utilities|Array|Add (LocalVariables|GetL_GridArray) _array_element_2)
            (if (not (Utilities|Array|ContainsItem (.gridpoint (.Value (Utilities|Map|Find (LocalVariables|GetL_DebuggedPoints) _array_element_2))) _array_element))
              (if (Utilities|Array|ContainsItem (TravelPoints|GetTravelablePoints _array_element_2) _array_element)
                (Rendering|Debug|DrawDebugLine (+ (LocalVariables|GetL_Offset) (Transformation|GetActorLocation _array_element)) (+ (LocalVariables|GetL_Offset) (Transformation|GetActorLocation _array_element_2)) "(R=1.000000,G=1.000000,B=1.000000,A=1.000000)" 5.0 5.0)
                (else
                  (Rendering|Debug|DrawDebugArrow (+ (LocalVariables|GetL_Offset) (Transformation|GetActorLocation _array_element)) (+ (LocalVariables|GetL_Offset) (Transformation|GetActorLocation _array_element_2)) 3e+02 "(R=1.000000,G=1.000000,B=0.000000,A=1.000000)" 5.0 5.0)))))))
      (Utilities|Map|Add (LocalVariables|GetL_DebuggedPoints) _array_element (Utilities|Struct|MakeS_GridPointArray (LocalVariables|GetL_GridArray))))))

(fn GetTravelablePoints
  ;[0.15 0.15 0.15 0.5] GetTravelablePoints
  (return (Variables|TravelPoints|GetTravelablePoints)))

(fn ToggleContains
  (params (Condition :type Boolean) (Item :type BP%20Grid%20Point%20Object%20Reference%20%28by%20ref%29))
  ;[0.15 0.15 0.15 0.5] Toggles if an item contains (Needed due to utility blueprint not being able to edit inside its scope)
  (if Condition
    (Utilities|Array|RemoveItem (Variables|TravelPoints|GetTravelablePoints) Item)
    (else
      (Utilities|Array|AddUnique (Variables|TravelPoints|GetTravelablePoints) Item)))
  (return))