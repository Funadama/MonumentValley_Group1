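; BP_CodeAnimator is an actor that, on its first activation only, animates from its starting transform to EndPosition and rewires walkable tile links.
; A timeline lerps the transform, with start and finish dispatchers fired around it.
; Handlers bound to those dispatchers toggle both directions of each grid point link in StartTileLink and EndTileLink, so tile connections change as the piece leaves and arrives.
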(event Custom|OnAnimationFinished_Event
  ;[0.15 0.15 0.15 0.5] TileLink for when the animation starts, and stops
  (for _array_element (Variables|Animator|GetEndTileLink)
    (Default|ToggleContains (.gridpoint _array_element) (.link _array_element) (.linkto _array_element))
    (Default|ToggleContains (.linkto _array_element) (.link _array_element) (.gridpoint _array_element))))

(event Custom|OnAnimationStart_event
  ;[0.15 0.15 0.15 0.5] TileLink for when the animation starts, and stops
  (for _array_element (Variables|Animator|GetStartTileLink)
    (Default|ToggleContains (.gridpoint _array_element) (.link _array_element) (.linkto _array_element))
    (Default|ToggleContains (.linkto _array_element) (.link _array_element) (.gridpoint _array_element))))

(event EventBeginPlay
  ;[0.15 0.15 0.15 0.5] Get start position + bind events
  (Variables|Animator|SetBeginPosition (Transformation|GetActorTransform))
  (EventDispatchers|BindEventtoOnAnimationFinished (EventDispatchers|CreateEvent :!event Custom|OnAnimationFinished_Event))
  (EventDispatchers|BindEventtoOnAnimationStart (EventDispatchers|CreateEvent :!event Custom|OnAnimationStart_event)))

(event EventActivated
  ;[0.15 0.15 0.15 0.5] Start Animation, Lerp to the end position
  (Utilities|FlowControl|DoOnce false
    (:Completed
      (Default|CallOnAnimationStart)
      (bind _time (Timeline|Animation PlayFromStart)
        (:Update
          (Transformation|SetActorTransform (Math|Transform|Lerp(Transform) (Variables|Animator|GetBeginPosition) (Variables|Animator|GetEndPosition) _time)))
        (:Finished
          (Default|CallOnAnimationFinished))))))

(fn ConstructionScript)