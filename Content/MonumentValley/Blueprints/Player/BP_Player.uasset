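; Player actor for a Monument Valley-style puzzle game that walks along paths of connected grid nodes, including across optical-illusion gaps.
; FollowPathing starts looping timers; the step function moves by distance, slerping rotation to each node's up vector.
; Node arrivals fire a dispatcher that attaches the player to the node, truncates broken paths and teleports across large gaps.
; Movement audio volume follows the player's vertical screen position.
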(event Custom|OnMovementFinished_Event
  (bind _followingpath (Variables|Movement|GetFollowingPath))
  ;[0.15 0.15 0.15 0.5] Cancels the current movement.
  (Utilities|Time|ClearandInvalidateTimerbyHandle (Variables|Movement|GetAudioFadingTimer))
  (Utilities|Time|ClearandInvalidateTimerbyHandle (Variables|Movement|GetAudioFadingTimer))
  (Variables|Movement|SetGoingToNode 0)
  (Variables|Player|SetCurrentPosition (Utilities|Array|Get(acopy) _followingpath (Utilities|Array|LastIndex _followingpath)))
  (Utilities|Array|Clear (Variables|Movement|GetFollowingPath))
  (Audio|Components|Audio|Stop (Variables|Default|GetAudioSource)))

(event Custom|OnProcessNextNode_Event
  ;[0.15 0.15 0.15 0.5] Events that get triggered when the player reaches the next node.
  (if (Utilities|Array|IsValidIndex (Variables|Movement|GetFollowingPath) (Variables|Movement|GetGoingToNode))
    (Transformation|AttachActorToActor (Utilities|Array|Get(acopy) (Variables|Movement|GetFollowingPath) (Variables|Movement|GetGoingToNode)) "None" "KeepWorld" "KeepWorld" "KeepWorld" true)
    (bind _removednodes (Pathing|ProcessInvalidConnection))
    (if (not _removednodes)
      (bind (_skippednode _newposition) (Pathing|ProcessTeleport (Transformation|GetActorLocation (Getters|GetCurrentNode))))
      (if _skippednode
        (Transformation|SetActorLocation _newposition false false)
        (Default|CallOnProcessNextNode)))))

(event EventBeginPlay
  ;[0.15 0.15 0.15 0.5] Connect dispatchers
  (EventDispatchers|BindEventtoOnMovementFinished (EventDispatchers|CreateEvent :!event Custom|OnMovementFinished_Event))
  (EventDispatchers|BindEventtoOnProcessNextNode (EventDispatchers|CreateEvent :!event Custom|OnProcessNextNode_Event)))

(fn ConstructionScript)

(fn DebugPathing
  ;[0.15 0.15 0.15 0.5] Editor testing Code to Find valid paths
  (bind (_found _path) (CallFunction|FindPathing (Variables|Player|GetCurrentPosition) (Variables|Player|GetDebugTravelPoint)))
  (if _found
    (CallFunction|PrintDebugPath _path)
    (return)
    (else
      (return))))

(fn GetCurrentNode
  (bind _goingtonode (Variables|Movement|GetGoingToNode))
  (bind _followingpath (Variables|Movement|GetFollowingPath))
  (bind _returnvalue (- _goingtonode 1))
  (bind _returnvalue_2 (Math|Integer|Max(Integer) _returnvalue))
  ;[0.15 0.15 0.15 0.5] Gets the grid point position of the player, if the player is moving return the last point
  (if (not (Utilities|Array|IsValidIndex _followingpath _returnvalue_2))
    (return (Variables|Player|GetCurrentPosition))
    (else
      (return (Utilities|Array|Get(acopy) _followingpath _returnvalue_2)))))

(fn FollowPathing
  (params (Path :type Array%20of%20BP%20Grid%20Point%20Object%20References))
  (bind _audiosource (Variables|Default|GetAudioSource))
  (bind _output (Utilities|Array|Get(acopy) Path 1))
  (bind _output_2 (Utilities|Array|Get(acopy) Path))
  ;[0.15 0.15 0.15 0.5] Makes the player start following the path. If the player is between the first and second point, ignore the first so the player doesn't have to backtrack.
  (CallFunction|PrintDebugPath Path)
  (Variables|Movement|SetFollowingPath Path)
  (if (== _output_2 _output)
    (Variables|Movement|SetGoingToNode 0)
    (else
      (Variables|Movement|SetGoingToNode (Math|Integer|SelectInt 1 0 (CallFunction|IsVectorBetweenPoints (Transformation|GetActorLocation _output_2) (Transformation|GetActorLocation _output) (Transformation|GetActorLocation) (LocalVariables|GetL_ReturnDistance))))))
  (Default|CallOnProcessNextNode)
  (if (Audio|Components|Audio|IsPlaying _audiosource)
    _
    (else
      (Audio|Components|Audio|Play _audiosource 0.0)
      (bind _returnvalue (Utilities|Time|SetTimerbyEvent (EventDispatchers|CreateEvent :!event TickAudioFading) 0.05 true true))
      (Variables|Movement|SetAudioFadingTimer _returnvalue)))
  (bind _returnvalue_2 (Utilities|Time|SetTimerbyEvent (EventDispatchers|CreateEvent :!event TickStepNextPosition) 0.01 true true))
  (Variables|Movement|SetAudioFadingTimer _returnvalue_2)
  (return))

(fn TickStepNextPosition
  ;[0.15 0.15 0.15 0.5] Gets the Position, and distance to move.
  (LocalVariables|SetL_PlayerPosition (Transformation|GetActorLocation))
  (bind _output_get (LocalVariables|SetL_StepSize (* (Variables|Player|GetMovementSpeed) (Utilities|Time|GetWorldDeltaSeconds))))
  ;[0.15 0.15 0.15 0.5] While loop to calculate the position, and rotation for this tick
  (while (> _output_get 0.0)
    (if (Getters|IsNextNodeValid)
      ;[0.15 0.15 0.15 0.5] The position is calculated in steps. If the step size is greater than the distance to the next point, it will step to the next point.
      (bind (_position _excessivelength) (CallFunction|StepTowards (LocalVariables|GetL_PlayerPosition) (Getters|GetNextNodePosition) (LocalVariables|GetL_StepSize)))
      (LocalVariables|SetL_PlayerPosition _position)
      (LocalVariables|SetL_StepSize _excessivelength)
      (if (> _excessivelength 0.0)
        (Math|Integer|IncrementInt (Variables|Movement|GetGoingToNode)
          (:%20%20
            ;[0.15 0.15 0.15 0.5] Processes features for valid connections and skipping nodes. (The position is requested again due to changing in the dispatchers.)
            (Default|CallOnProcessNextNode)
            (LocalVariables|SetL_PlayerPosition (Transformation|GetActorLocation)))))
      (else
        (Default|CallOnMovementFinished)
        (LocalVariables|SetL_StepSize 0.0))))
  ;[0.15 0.15 0.15 0.5] Sets the position and rotation. It calculates the rotation based on the floor and direction to create a smooth feel.
  (Transformation|SetActorLocation (LocalVariables|GetL_PlayerPosition) false false)
  (if (Getters|IsNextNodeValid)
    (Transformation|SetActorRotation (Class|KismetMathLibrary|QuatRotator (Class|KismetMathLibrary|QuatSlerp (Math|Conversions|ToQuaternion(Rotator) (Transformation|GetActorRotation)) (Math|Conversions|ToQuaternion(Rotator) (Math|Rotator|MakeRotfromXZ (- (LocalVariables|GetL_PlayerPosition) (Getters|GetNextNodePosition)) (Transformation|GetActorUpVector (Utilities|Array|Get(acopy) (Variables|Movement|GetFollowingPath) (Variables|Movement|GetGoingToNode))))) (* (Variables|Player|GetRotationSpeed) (Utilities|Time|GetWorldDeltaSeconds)))))
    (return)
    (else
      (return))))

(fn GetNextNodePosition
  ;[0.15 0.15 0.15 0.5] Gets the position of the next node.
  (return (Transformation|GetActorLocation (Utilities|Array|Get(acopy) (Variables|Movement|GetFollowingPath) (Variables|Movement|GetGoingToNode)))))

(fn ProcessTeleport
  (params (PlayerPosition :type Vector))
  ;[0.15 0.15 0.15 0.5] A check for when to skip a node, to handle optical illusions.
  (if (Getters|IsNextNodeValid)
    (bind _output_get (LocalVariables|SetL_SavedPosition (Getters|GetNextNodePosition)))
    (if (>= (Math|Vector|Distance(Vector) _output_get PlayerPosition) (LocalVariables|GetL_SkipDistance))
      (Math|Integer|IncrementInt (Variables|Movement|GetGoingToNode)
        (:%20%20
          (return true (LocalVariables|GetL_SavedPosition))))
      (else
        (return false PlayerPosition)))
    (else
      (return false PlayerPosition))))

(fn ProcessInvalidConnection
  (bind _gridpoint (Getters|GetCurrentNode))
  (bind _followingpath (Variables|Movement|GetFollowingPath))
  (bind _returnvalue (Utilities|Array|FindItem _followingpath _gridpoint))
  (bind _returnvalue_2 (+ _returnvalue 1))
  ;[0.15 0.15 0.15 0.5] Checks if the current and next index is valid.
  (LocalVariables|SetL_NextIndex _returnvalue_2)
  (if (Utilities|Array|IsValidIndex _followingpath _returnvalue_2)
    ;[0.15 0.15 0.15 0.5] Checks if the path between the current and next nodes is still connected. (If they’re not, remove all the next indices.)
    (if (Utilities|Array|ContainsItem (Default|GetTravelablePoints (Getters|GetCurrentNode)) (Utilities|Array|Get(acopy) (Variables|Movement|GetFollowingPath) (LocalVariables|GetL_NextIndex)))
      (return false)
      (else
        (bind _output_get (LocalVariables|SetL_AmountToRemove (- (Utilities|Array|Length (Variables|Movement|GetFollowingPath)) _returnvalue)))
        (for _index (range 0 _output_get)
          (Utilities|Array|RemoveIndex (Variables|Movement|GetFollowingPath) (LocalVariables|GetL_NextIndex)))
        (return true)))
    (else
      (return false))))

(fn IsNextNodeValid
  ;[0.15 0.15 0.15 0.5] IsNextNodeValid
  (return (Utilities|Array|IsValidIndex (Variables|Movement|GetFollowingPath) (Variables|Movement|GetGoingToNode))))

(fn TickAudioFading
  ;[0.15 0.15 0.15 0.5] Updates the AudioSource's volume multiplier depending on the vertical position of the player
  (Audio|Components|Audio|SetVolumeMultiplier (Variables|Default|GetAudioSource) (Math|Float|MapRangeClamped (* (/ 1e+02 (.y (Viewport|GetViewportSize))) (.y (.ScreenPosition (Class|GameplayStatics|ProjectWorldtoScreen (Game|GetPlayerController 0) (Transformation|GetActorLocation) false)))) 3e+01 8e+01 0.25 1.5) :!class /Script/Engine.AudioComponent)
  (return))