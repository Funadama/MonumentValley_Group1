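; Touch-interactable actor that the player rotates around a configurable axis, snapping to angle multiples on release.
; Touches are projected onto a camera-facing plane through the actor's origin, and the change in signed angle drives local rotation.
; On release, a timeline eases to the nearest snap angle with interaction disabled.
; The rotation-state dispatcher fires on touch, then after snapping with the state looked up from a map.
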(event EventInteractableTouchOngoing
  (params (RawInputPos :type Vector%202D%20Structure))
  (bind _returnvalue (Math|GetTouchAngle RawInputPos))
  ;[0.15 0.15 0.15 0.5] Updates the rotation of the actor
  (RotationSetting|AddAngletoAxis (Variables|Config|GetRotationAxis) (- _returnvalue (Variables|Internal|GetCurrentAngle)))
  (Variables|Internal|SetCurrentAngle _returnvalue))

(event EventInteractableTouchReleased
  (bind _snapanglemultiple (Variables|Snapping|GetSnapAngleMultiple))
  (bind _rotationaxis (Variables|Config|GetRotationAxis))
  (bind _returnvalue (Getters|GetAxisValue _rotationaxis))
  (bind _returnvalue_2 (/ _returnvalue _snapanglemultiple))
  (bind _returnvalue_3 (Math|Float|Round _returnvalue_2))
  ;[0.15 0.15 0.15 0.5] Snaps the actor's rotation to the closest angle specified in the SnapAngleMultiple variable
  (Variables|Conditions|SetIsActive false)
  (Variables|Snapping|SetRotationStateAfterSnapping (.Value (Utilities|Map|Find (Variables|Snapping|GetRotationStateMap) _returnvalue_3)))
  (Variables|Snapping|SetSnapAngle (* (Variables|Snapping|GetSnapAngleMultiple) _returnvalue_3))
  ;;[0 0 0 0.5] Rotates the released actor towards the nearest 90 degree angle
  (bind _angleprogression (Timeline|Timeline PlayFromStart)
    (:Update
      (Variables|Snapping|SetRotationSnapDeltaTime (+ (Variables|Snapping|GetRotationSnapDeltaTime) _angleprogression))
      (RotationSetting|SetAxisValue (Variables|Config|GetRotationAxis) (Math|Interpolation|FInterpTo (Getters|GetAxisValue (Variables|Config|GetRotationAxis)) (Variables|Snapping|GetSnapAngle) (Variables|Snapping|GetRotationSnapDeltaTime) 1.0)))
    (:Finished
      ;;[0 0 0 0.5] Enables the interaction, resets the deltaTime and calls the dispatcher with the new rotation state
      (Variables|Conditions|SetIsActive true)
      (Variables|Snapping|SetRotationSnapDeltaTime 0.0)
      (Default|CallOnRotationStateChanged (Variables|Snapping|GetRotationStateAfterSnapping)))))

(fn ConstructionScript)

(fn GetDirectionTowardsCamera
  ;[0.15 0.15 0.15 0.5] Gets the normalized direction from the actor to the camera
  (return (Math|Vector|GetUnitDirection(Vector) (Transformation|GetActorLocation) (Camera|GetCameraLocation (Game|GetPlayerCameraManager 0)))))

(fn GetAxisValue
  (params (Axis :type E_RotationAxis%20Enum :default "NewEnumerator0"))
  (bind _returnvalue (Transformation|GetActorRotation))
  ;[0.15 0.15 0.15 0.5] Gets the rotation value of the given axis
  (return (Utilities|Select :Index Axis :NewEnumerator0 0.0 :NewEnumerator1 (.roll _returnvalue) :NewEnumerator2 (.pitch _returnvalue) :NewEnumerator3 (.yaw _returnvalue))))

(fn ProjectInputonPlane
  (params (ScreenPosition :type Vector%202D%20Structure%20%28by%20ref%29))
  ;[0.15 0.15 0.15 0.5] Gets the position of the input as if it was on the same plane as the actor
  (return (Class|KismetMathLibrary|ProjectPointontoPlane (.WorldPosition (Class|GameplayStatics|DeprojectScreentoWorld (Game|GetPlayerController 0) ScreenPosition)) (Transformation|GetActorLocation) (Getters|GetDirectionTowardsCamera))))

(fn GetTouchAngle
  (params (ScreenPosition :type Vector%202D%20Structure%20%28by%20ref%29))
  (bind _normal (Getters|GetDirectionTowardsCamera))
  (bind _returnvalue (Transformation|GetActorLocation))
  (bind _positiononactorplane (Getters|ProjectInputonPlane ScreenPosition))
  (bind _returnvalue_2 (Math|Rotator|MakeRotfromX _normal))
  (bind _returnvalue_3 (Math|Vector|GetRightVector _returnvalue_2))
  (bind _returnvalue_4 (Math|Vector|GetUnitDirection(Vector) _returnvalue _positiononactorplane))
  (bind _returnvalue_5 (Math|Vector|DotProduct _returnvalue_3 _returnvalue_4))
  (bind _returnvalue_6 (Class|KismetMathLibrary|DegAcos _returnvalue_5))
  ;[0.15 0.15 0.15 0.5] Gets the angle of the touch position projected on a plane projected from the actor's origin facing the camera
  (return (Math|Float|SelectFloat _returnvalue_6 (* _returnvalue_6 -1.0) (< (Math|Vector|DotProduct (Math|Vector|GetUpVector _returnvalue_2) _returnvalue_4) 0.0))))

(fn AddAngletoAxis
  (params (Axis :type E_RotationAxis%20Enum :default "NewEnumerator0") (Angle :type Float%20%28double-precision%29))
  ;[0.15 0.15 0.15 0.5] Adds the given angle to the given axis's value
  (switch Utilities|FlowControl|Switch|SwitchonE_RotationAxis Axis
    (:NewEnumerator0
      _)
    (:NewEnumerator1
      (Transformation|AddActorLocalRotation (Math|Rotator|MakeRotator Angle 0.0 0.0) false false))
    (:NewEnumerator2
      (Transformation|AddActorLocalRotation (Math|Rotator|MakeRotator 0.0 Angle 0.0) false false))
    (:NewEnumerator3
      (Transformation|AddActorLocalRotation (Math|Rotator|MakeRotator 0.0 0.0 (* Angle -1.0)) false false)))
  (return))

(fn SetAxisValue
  (params (Axis :type E_RotationAxis%20Enum :default "NewEnumerator0") (Angle :type Float%20%28double-precision%29))
  (bind _returnvalue (Transformation|GetActorRotation))
  (bind _returnvalue_2 (Transformation|GetActorRotation))
  (bind _returnvalue_3 (Transformation|GetActorRotation))
  ;[0.15 0.15 0.15 0.5] Sets the rotational angle on the given axis
  (Transformation|SetActorRotation (Utilities|Select :Index Axis :NewEnumerator0 "0, 0, 0" :NewEnumerator1 (Math|Rotator|MakeRotator Angle (.pitch _returnvalue_2) (.yaw _returnvalue_2)) :NewEnumerator2 (Math|Rotator|MakeRotator (.roll _returnvalue_3) Angle (.yaw _returnvalue_3)) :NewEnumerator3 (Math|Rotator|MakeRotator (.roll _returnvalue) (.pitch _returnvalue) Angle)))
  (return))

(fn InteractableonTouched
  (params (ImpactPoint :type Vector :default "0, 0, 0") (RawInputPos :type Vector%202D%20Structure))
  ;[0.15 0.15 0.15 0.5] Returns that it is a valid interactable and saves the starting angle between the base and
  (if (Variables|Conditions|GetIsActive)
    (Variables|Internal|SetCurrentAngle (Math|GetTouchAngle RawInputPos))
    (Default|CallOnRotationStateChanged "NewEnumerator0")
    (return true)
    (else
      (return false))))