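; GameManager routes player click-to-move in the Monument Valley project, linking camera selection to player movement.
; On BeginPlay it finds BP_CameraPawn and BP_Player and binds to the camera pawn's selected-actor-changed event.
; When the selection is a BP_GridPoint, it runs FindPathing from the player's current node and sends any found path to the player to follow.
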(event EventBeginPlay
  ;[0.15 0.15 0.15 0.5] Binds events, and gets refs
  (bind _returnvalue (Actor|GetActorOfClass "/Game/MonumentValley/Blueprints/Pawn/BP_CameraPawn.BP_CameraPawn_C"))
  (bind _output_get (Variables|ActorComponents|SetBP_CameraPawn _returnvalue))
  (EventDispatchers|BindEventtoOnSelectedActorChanged _output_get (EventDispatchers|CreateEvent :!event OnSelectedActorChanged))
  (bind _returnvalue_2 (Actor|GetActorOfClass "/Game/MonumentValley/Blueprints/Player/BP_Player.BP_Player_C"))
  (Variables|ActorComponents|SetBP_Player _returnvalue_2))

(fn ConstructionScript)

(fn OnSelectedActorChanged
  (params (SelectedActor :type Actor%20Object%20Reference))
  ;[0.15 0.15 0.15 0.5] Sets an event for the player when the grid point is interacted with.
  (bind _asbp_grid_point (Utilities|Casting|CastToBP_GridPoint SelectedActor)
    (:then
      (bind (_found _path) (CallFunction|FindPathing (Default|GetCurrentNode (Variables|ActorComponents|GetBP_Player)) _asbp_grid_point))
      (if _found
        (Default|FollowPathing (Variables|ActorComponents|GetBP_Player) _path)
        (return)
        (else
          (return))))
    (:CastFailed
      (return))))