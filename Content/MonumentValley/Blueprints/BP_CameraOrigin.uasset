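; BP_CameraOrigin is the focal point that creates and positions the player's camera in the Monument Valley project.
; On BeginPlay it spawns a BP_CameraPawn, has player controller 0 possess it, and attaches it to itself keeping world transforms.
; GetCameraTransform rotates the origin's forward vector by CameraAngle, offsets it by DistanceFromOrigin, and aims the camera back at the origin with a look-at rotation.
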(event EventBeginPlay
  ;[0.15 0.15 0.15 0.5] Spawns the camera pawn at the correct position and sets it as the main player
  (bind _returnvalue (Game|SpawnActorfromClass "/Game/MonumentValley/Blueprints/BP_CameraPawn.BP_CameraPawn_C" (CallFunction|GetCameraTransform) "Undefined" "MultiplyWithRoot" 0 0))
  (Pawn|Possess (Game|GetPlayerController 0) _returnvalue)
  (Transformation|AttachActorToActor _returnvalue self "None" "KeepWorld" "KeepWorld" "KeepWorld" true))

(fn ConstructionScript)

(fn GetCameraTransform
  (bind _returnvalue (Transformation|GetActorForwardVector))
  (bind _returnvalue_2 (Transformation|GetActorLocation))
  (bind _distancefromorigin (Variables|Config|GetDistanceFromOrigin))
  (bind _cameraangle (Variables|Internal|GetCameraAngle))
  (bind _returnvalue_3 (Math|Vector|RotateVector _returnvalue _cameraangle))
  (bind _returnvalue_4 (* _returnvalue_3 _distancefromorigin))
  (bind _returnvalue_5 (+ _returnvalue_2 _returnvalue_4))
  ;[0.15 0.15 0.15 0.5] Gets the required transform of the player's camera
  (return (Math|Transform|MakeTransform _returnvalue_5 (Math|Rotator|FindLookatRotation _returnvalue_5 (Transformation|GetActorLocation)))))